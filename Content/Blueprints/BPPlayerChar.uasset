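; Player character Blueprint that drives its own movement along a continuously changing pitch direction.
; BeginPlay caches the capsule's world rotation as a base rotator.
; Each Tick, after a successful ARGameInstance cast, it increments that rotator's pitch and feeds its forward vector into AddMovementInput.
; The branch is hardwired true and the game instance's GetUp is unused, so the game instance does not steer movement.
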(event EventBeginPlay
  (Variables|Default|SetBase%20ROtator (Transformation|GetWorldRotation (Variables|Collision|GetCapsuleComponent))))

(event Collision|EventActorBeginOverlap
  (params (OtherActor :type Actor%20Object%20Reference)))

(event EventTick
  (params (DeltaSeconds :type Float%20%28single-precision%29))
  (bind _asargame_instance (Utilities|Casting|CastToARGameInstance (Game|GetGameInstance)))
  (if true
    (bind _result (Math|Float|IncrementFloat (.Pitch (Math|Rotator|BreakRotator (Variables|Default|GetBase%20ROtator))))
      (:%20%20
        (bind _output_get (Variables|Default|SetBase%20ROtator (Math|Rotator|MakeRotator (.Roll (Math|Rotator|BreakRotator (Variables|Default|GetBase%20ROtator))) _result (.Yaw (Math|Rotator|BreakRotator (Variables|Default|GetBase%20ROtator))))))
        (Pawn|Input|AddMovementInput (Math|Rotator|GetRotationXVector _output_get) 1.0 false)))))

(fn ConstructionScript)