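; BP_Player is the player pawn, which moves forward automatically while the game is in its racing state.
; Each tick it reads the racing state from ARGameInstance and, when active, adds full movement input along the control rotation's yaw, keeping movement horizontal.
; It also applies the game instance's Up and Right values as controller pitch and yaw, so steering comes from that shared object rather than input events in this Blueprint.
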(event EventTick
  (params (DeltaSeconds :type Float%20%28single-precision%29))
  (bind _returnvalue (Game|GetGameInstance))
  (bind _asargame_instance (Utilities|Casting|CastToARGameInstance (Game|GetGameInstance)))
  (if (Class|ARGameInstance|GetRacingState _asargame_instance)
    (Pawn|Input|AddMovementInput (Math|Vector|GetForwardVector (Math|Rotator|MakeRotator 0.0 0.0 (.yaw (Pawn|GetControlRotation :!class /Script/Engine.Pawn)))) 1.0 false)
    (bind _asargame_instance_2 (Utilities|Casting|CastToARGameInstance _returnvalue))
    (Pawn|Input|AddControllerPitchInput (Class|ARGameInstance|GetUp _asargame_instance_2))
    (bind _asargame_instance_3 (Utilities|Casting|CastToARGameInstance _returnvalue))
    (Pawn|Input|AddControllerYawInput (Class|ARGameInstance|GetRight _asargame_instance_3))))

(fn ConstructionScript)