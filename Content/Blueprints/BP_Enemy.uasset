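; BP_Enemy is an AI racer that moves between checkpoints along a quadratic Bezier curve.
; While racing, a checkpoint trigger from ARGameInstance makes it fetch the next point, transform it by the actor transform, derive a third point and play a timeline after a short delay.
; The timeline update logic sets location through nested lerps, rotation from a finite-difference tangent, and draws a debug trail.
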(event EventTick
  (params (DeltaSeconds :type Float%20%28single-precision%29))
  (bind _asargame_instance (Utilities|Casting|CastToARGameInstance (Game|GetGameInstance)))
  (if (Class|ARGameInstance|GetRacingState _asargame_instance)
    ;[1 1 1] Did we just hit a check point
    (if (Class|ARGameInstance|GetAiBoxTrigger _asargame_instance)
      (Class|ARGameInstance|SetAiBoxTrigger _asargame_instance false)
      (Variables|Default|SetStart (Transformation|GetActorLocation))
      (Variables|Default|SetPoint%201 (.Location (Math|Transform|BreakTransform (Class|ARGameInstance|GetNextPoint _asargame_instance))))
      (CallFunction|UpdatetoWorldVector (Variables|Default|GetPoint%201))
      (Variables|Default|SetPoint%202 (+ (+ (Variables|Default|GetStart) (/ (- (Variables|Default|GetStart) (Variables|Default|GetPoint%201)) 2)) (Math|Vector|MakeVector 0.0 0.0 (.Z (Math|Vector|BreakVector (/ (- (Variables|Default|GetStart) (Variables|Default|GetPoint%201)) 2))))))
      (Utilities|FlowControl|Delay 0.2)
      (Components|Timeline|PlayfromStart (Variables|Default|GetTimeline_Lerp)))))

(fn ConstructionScript)

(fn GetLocationBeziar
  (params (Start :type Vector) (End :type Vector) (Anchor :type Vector) (Time :type Float%20%28single-precision%29))
  (Utilities|FlowControl|Sequence
    (:then_0
      (LocalVariables|SetTemp%20A (Math|Vector|Lerp(Vector) Start End Time))
      (LocalVariables|SetTemp%20B (Math|Vector|Lerp(Vector) End Anchor Time)))
    (:then_1
      (return (Math|Vector|Lerp(Vector) (LocalVariables|GetTemp%20A) (LocalVariables|GetTemp%20B) Time)))))

(fn GetRotationBeziar0
  (params (Start :type Vector) (End :type Vector) (Anchor :type Vector) (Time :type Float%20%28single-precision%29))
  (bind _returnvalue (+ Time -0.001))
  (LocalVariables|SetTemp%20Current (CallFunction|GetLocationBeziar Start End Anchor Time))
  (if (Math|Float|InRange(Float) _returnvalue 0.0 1.0)
    (return (Math|Conversions|RotationFromXVector (Math|Vector|Normalize (- (LocalVariables|GetTemp%20Current) (CallFunction|GetLocationBeziar Start End Anchor _returnvalue)))))
    (else
      (return (Math|Conversions|RotationFromXVector (Math|Vector|Normalize (- (LocalVariables|GetTemp%20Current) (CallFunction|GetLocationBeziar Start End Anchor (+ Time 0.001)))))))))

(fn UpdatetoWorldVector
  (params (Input :type Vector%20%28by%20ref%29))
  (|SetBy-RefVar Input (Math|Transform|TransformLocation (Transformation|GetActorTransform) Input)))